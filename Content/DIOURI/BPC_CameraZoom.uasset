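; Camera zoom component for the RTS player character, driving its spring arm's length and pitch from the mouse wheel.
; Each wheel notch steps a zoom multiplier and a wanted pitch angle, both clamped to bounds.
; Every tick interpolates the arm toward those targets, zeroing relative yaw and roll.
; A tiny box overlap at the camera resets the multiplier to a fixed value on hitting WorldStatic objects.
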(event `self.ReceiveBeginPlay`
  (bind (_returnvalue_roll _returnvalue_pitch _returnvalue_yaw) (`KismetMathLibrary.BreakRotator` (`SpringArmComponent.GetTargetRotation` (`self.Spring Arm`))))
  ;[1 1 1] CameraZoom
  (bind _asbp_nd_rtsplayer_character (cast `/Game/DIOURI/BP_ND_RTSPlayerCharacter` (`GameplayStatics.GetPlayerCharacter` 0)))
  (bind _output_get (set `self.As BP ND RTSPlayer Character` _asbp_nd_rtsplayer_character))
  (bind _output_get_2 (set `self.Spring Arm` (`/Game/DIOURI/BP_ND_RTSPlayerCharacter.SpringArm` _output_get)))
  (set `SpringArmComponent.TargetArmLength` (* (`self.ZoomStep`) (`self.ZooomMultiplier`)) _output_get_2)
  (set `self.CurrentZAngle` _returnvalue_yaw))

(event `self.ReceiveTick`
  (params (DeltaSeconds :type "Float (single-precision)"))
  ;[1 1 1] CameraZoom
  (`self.UpdateCameraZoom`)
  (bind (_outactors _returnvalue) (`KismetSystemLibrary.BoxOverlapActors` (`SceneComponent.K2_GetComponentLocation` (`/Game/DIOURI/BP_ND_RTSPlayerCharacter.Camera` (stale `self.ReceiveBeginPlay` _output_get))) (1.0 1.0 1.0) (`|MakeArray` "ObjectTypeQuery1" :!type "EObjectTypeQuery Enum")))
  (if _returnvalue
    (set `self.ZooomMultiplier` 12.0)))

(event `Key|MouseScrollDown`
  (params (Key :type "Key Structure"))
  (bind (_yzoombounds_x _yzoombounds_y) (`KismetMathLibrary.BreakVector2D` (`self.YZoomBounds`)))
  (bind (_zoombounds_x _zoombounds_y) (`KismetMathLibrary.BreakVector2D` (`self.ZoomBounds`)))
  ;[1 1 1] CameraZoom
  (:`Pressed`
    (`/Engine/EditorBlueprintResources/StandardMacros.DecrementFloat` (`self.WantedAngle`)
      (:`  `
        (`/Engine/EditorBlueprintResources/StandardMacros.IncrementFloat` (`self.ZooomMultiplier`)
          (:`  `
            (set `self.ZooomMultiplier` (`KismetMathLibrary.FClamp` (`self.ZooomMultiplier`) _zoombounds_x _zoombounds_y))
            (set `self.WantedAngle` (`KismetMathLibrary.FClamp` (`self.WantedAngle`) _yzoombounds_y _yzoombounds_x))))))))

(event `Key|MouseScrollUp`
  (params (Key :type "Key Structure"))
  (bind (_yzoombounds_x _yzoombounds_y) (`KismetMathLibrary.BreakVector2D` (`self.YZoomBounds`)))
  (bind (_zoombounds_x _zoombounds_y) (`KismetMathLibrary.BreakVector2D` (`self.ZoomBounds`)))
  ;[1 1 1] CameraZoom
  (:`Pressed`
    (`/Engine/EditorBlueprintResources/StandardMacros.IncrementFloat` (`self.WantedAngle`)
      (:`  `
        (`/Engine/EditorBlueprintResources/StandardMacros.DecrementFloat` (`self.ZooomMultiplier`)
          (:`  `
            (set `self.ZooomMultiplier` (`KismetMathLibrary.FClamp` (`self.ZooomMultiplier`) _zoombounds_x _zoombounds_y))
            (set `self.WantedAngle` (`KismetMathLibrary.FClamp` (`self.WantedAngle`) _yzoombounds_y _yzoombounds_x))))))))

(fn `UpdateCameraZoom`
  (bind (_returnvalue_roll _returnvalue_pitch) (`KismetMathLibrary.BreakRotator` (`SpringArmComponent.GetTargetRotation` (`self.Spring Arm`))))
  (set `self.CurrentZoom` (`SpringArmComponent.TargetArmLength` (`self.Spring Arm`)))
  (set `self.CurrentYZoom` _returnvalue_pitch)
  (set `SpringArmComponent.TargetArmLength` (`KismetMathLibrary.FInterpTo` (`self.CurrentZoom`) (+ (* (`self.ZoomStep`) (`self.ZooomMultiplier`)) 1500.0) (`GameplayStatics.GetWorldDeltaSeconds`) 20.0) (`self.Spring Arm`))
  (`SceneComponent.K2_SetRelativeRotation` (`self.Spring Arm`) (`KismetMathLibrary.MakeRotator` 0.0 (`KismetMathLibrary.FInterpTo` (`self.CurrentYZoom`) (`self.WantedAngle`) (`GameplayStatics.GetWorldDeltaSeconds`) 20.0)) false false))