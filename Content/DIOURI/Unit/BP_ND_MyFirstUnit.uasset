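; Unit character that chases and attacks a target, with speed, attack, health, armor and range stats copied from ActualUnit in the construction script.
; SetAttacking stores or clears the target, then attacks if within range or otherwise moves toward it with AIMoveTo.
; Tick stops movement and enters the attack loop whenever a valid target is in range.
; The loop repeats on an attack-speed Delay, subtracting damage directly from the target's DumyHealth.
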(event `self.ReceiveBeginPlay`)

(event `SetAttacking`
  (params (IsAttacking :type Boolean) (TargetToAtatack :type "/Game/DIOURI/Unit/BP_ND_Dumy Object Reference"))
  (bind _output_get (set `self.Target` TargetToAtatack))
  (if IsAttacking
    (if (<= (`KismetMathLibrary.Abs` (`KismetMathLibrary.VSize` (- (`SceneComponent.K2_GetComponentLocation` (`Character.Mesh` TargetToAtatack)) (`SceneComponent.K2_GetComponentLocation` (`self.CapsuleComponent`))))) (`self.UnitRange`))
      (`MovementComponent.StopMovementImmediately` (`self.CharacterMovement`))
      (set `self.IsAttacking` true :!label _label)
      (`KismetSystemLibrary.Delay` (`self.UnitAttackSpeed`) :!label _label_2)
      (if (`self.IsAttacking`)
        (set `/Game/DIOURI/Unit/BP_ND_Dumy.DumyHealth` (- (`/Game/DIOURI/Unit/BP_ND_Dumy.DumyHealth` _output_get) (`self.UnitAttackDamage`)) _output_get)
        (goto _label_2))
      (else
        (`|AIMoveTo` self (0.0 0.0 0.0) TargetToAtatack)))
    (else
      (set `self.IsAttacking` false)
      (set `self.Target` null))))

(event `self.ReceiveTick`
  (params (DeltaSeconds :type "Float (single-precision)"))
  (`self.Target`
    (:`then`
      (if (<= (`KismetMathLibrary.Abs` (`KismetMathLibrary.VSize` (- (`SceneComponent.K2_GetComponentLocation` (`Character.CapsuleComponent` (`self.Target`))) (`SceneComponent.K2_GetComponentLocation` (`self.CapsuleComponent`))))) (`self.UnitRange`))
        (`MovementComponent.StopMovementImmediately` (`self.CharacterMovement`))
        (goto _label)))
    (:`else`)))

(fn `UserConstructionScript`
  (set `self.UnitSpeed` (`/Game/DIOURI/Unit/BP_ND_MyFirstUnit.Speed` (`self.ActualUnit`)))
  (set `self.UnitAttackSpeed` (`/Game/DIOURI/Unit/BP_ND_MyFirstUnit.AttackSpeed` (`self.ActualUnit`)))
  (set `self.UnitAttackDamage` (`/Game/DIOURI/Unit/BP_ND_MyFirstUnit.AttackDamage` (`self.ActualUnit`)))
  (set `self.UnitHP` (`/Game/DIOURI/Unit/BP_ND_MyFirstUnit.HealthPoints` (`self.ActualUnit`)))
  (set `self.UnitArmor` (`/Game/DIOURI/Unit/BP_ND_MyFirstUnit.Armor` (`self.ActualUnit`)))
  (set `self.UnitRange` (`/Game/DIOURI/Unit/BP_ND_MyFirstUnit.Range` (`self.ActualUnit`)))
  (set `CharacterMovementComponent.MaxWalkSpeed` (`self.UnitSpeed`) (`self.CharacterMovement`)))