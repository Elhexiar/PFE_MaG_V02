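; RTS player controller that sets up the HUD, moves the camera and handles unit selection, orders and test keys for cards and an AOE event.
; Tick turns cursor position near screen edges into injected Enhanced Input vectors for the camera-move action.
; Left click starts HUD box drawing and selects a dummy, or ends area targeting.
; Right click drags a ghost unit, then orders selected units to attack a hovered dummy or AI-move with VFX.
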(event `self.ReceiveBeginPlay`
  (bind _asplayer_controller (cast `PlayerController` self))
  (bind _returnvalue (pcsubsystem `EnhancedInputLocalPlayerSubsystem` _asplayer_controller))
  (`/Engine/EditorBlueprintResources/StandardMacros.IsValid` _returnvalue
    (:`Is Valid`
      (`EnhancedInputSubsystemInterface.AddMappingContext` _returnvalue "/Game/DIOURI/Input/IC_ND_InputContext.IC_ND_InputContext" 0 (struct))
      ;[0.1875 0.1875 0.1875] Game HUD
      (bind _returnvalue_2 (`|CreateWidget` "/Game/DIOURI/UI/WBP_ND_CardHud.WBP_ND_CardHud_C"))
      (`UserWidget.AddToViewport` _returnvalue_2 0)
      (set `self.gameHUD` _returnvalue_2)
      (bind _asbp_nd_hud (cast `/Game/DIOURI/BP_ND_HUD` (`self.GetHUD`)))
      (set `self.BP HUD` _asbp_nd_hud)
      (bind _returnvalue_3 (`|GenericCreateObject` "/Game/DIOURI/UI/MainUI/WBP_UnitFinder.WBP_UnitFinder_C"))
      (`UserWidget.AddToViewport` _returnvalue_3 0))))

(event `EnhancedInput|/Game/DIOURI/Input/IA_ND_CameraMove`
  (params (ActionValue :type "Vector2D Structure") (ElapsedSeconds :type "Float (double-precision)") (TriggeredSeconds :type "Float (double-precision)") (InputAction :type "InputAction Object Reference" :default "/Game/DIOURI/Input/IA_ND_CameraMove.IA_ND_CameraMove"))
  (bind (_returnvalue_roll _returnvalue_pitch _returnvalue_yaw) (`KismetMathLibrary.BreakRotator` (`self.GetControlRotation`)))
  (bind (_returnvalue_roll_2 _returnvalue_pitch_2 _returnvalue_yaw_2) (`KismetMathLibrary.BreakRotator` (`self.GetControlRotation`)))
  ;[0.1875 0.1875 0.1875] Camera Movement
  (:`Triggered`
    (`Pawn.AddMovementInput` (`GameplayStatics.GetPlayerPawn` 0) (`KismetMathLibrary.GetRightVector` (`KismetMathLibrary.MakeRotator` _returnvalue_roll_2 0.0 _returnvalue_yaw_2)) ActionValue_X false)
    (`Pawn.AddMovementInput` (`GameplayStatics.GetPlayerPawn` 0) (`KismetMathLibrary.GetForwardVector` (`KismetMathLibrary.MakeRotator` 0.0 0.0 _returnvalue_yaw)) ActionValue_Y false)))

(event `Key|C`
  (params (Key :type "Key Structure"))
  ;[0.1875 0.1875 0.1875] Card Test
  (:`Pressed`
    (bind _returnvalue (`|CreateWidget` (`KismetArrayLibrary.Array_Random` (`self.deck`))))
    (set `/Game/DIOURI/Cards/ND_Cards.cardName` (`KismetStringLibrary.Concat_StrStr` "card" (`KismetStringLibrary.Conv_IntToString` (`self.cardCount`))) _returnvalue)
    (`HorizontalBox.AddChildToHorizontalBox` (`/Game/DIOURI/UI/WBP_ND_CardHud.HorizontalBox_0` (`self.gameHUD`)) _returnvalue)
    (bind _returnvalue_2 (`WidgetLayoutLibrary.SlotAsHorizontalBoxSlot` _returnvalue))
    (`HorizontalBoxSlot.SetSize` _returnvalue_2 (make `SlateChildSize` 1.0))
    (`HorizontalBoxSlot.SetHorizontalAlignment` _returnvalue_2 "HAlign_Center")
    (`HorizontalBoxSlot.SetVerticalAlignment` _returnvalue_2 "VAlign_Fill")
    (`/Engine/EditorBlueprintResources/StandardMacros.IncrementInt` (`self.cardCount`))))

(event `EnhancedInput|/Game/DIOURI/Input/IA_ND_MouseRightClick`
  (params (ActionValue :type Boolean) (ElapsedSeconds :type "Float (double-precision)") (TriggeredSeconds :type "Float (double-precision)") (InputAction :type "InputAction Object Reference" :default "/Game/DIOURI/Input/IA_ND_MouseRightClick.IA_ND_MouseRightClick"))
  (bind (_hit _location) (`self.Get location Under Cursor`))
  (bind (_hit_2 _location_2) (`self.Get location Under Cursor`))
  (:`Triggered`
    (`self.K2_SetActorLocation` (`self.UnitGhost`) _location_2 false false))
  (:`Started`
    (bind _returnvalue (`|SpawnActorFromClass` "/Game/DIOURI/Unit/BP_GhostUnit.BP_GhostUnit_C" (`KismetMathLibrary.MakeTransform` _location_2) "Undefined" "MultiplyWithRoot" null null))
    (set `self.UnitGhost` _returnvalue))
  (:`Completed`
    ;[0.1875 0.1875 0.1875] Right Click
    (`KismetSystemLibrary.LogString` "Hello")
    (bind _asbp_nd_dumy (cast `/Game/DIOURI/Unit/BP_ND_Dumy` (`.HitActor` (`GameplayStatics.BreakHitResult` (`self.GetHitResultUnderCursorByChannel` "TraceTypeQuery1"))))
      (:`then`
        (if (`/Game/DIOURI/Unit/BP_ND_Dumy.Hovering` _asbp_nd_dumy)
          (for _array_element (`self.SelectedUnitList`)
            (`/Game/DIOURI/Unit/BP_ND_MyFirstUnit.SetAttacking` _array_element true _asbp_nd_dumy))))
      (:`CastFailed`
        ;;[1 1 1] Spawn Move VFX
        (`NiagaraFunctionLibrary.SpawnSystemAtLocation` (`self.Move VFX`) _location)
        (for _array_element_2 (`self.SelectedUnitList`)
          (`/Game/DIOURI/Unit/BP_ND_MyFirstUnit.SetAttacking` _array_element_2 false null)
          (`|AIMoveTo` _array_element_2 _array_element_2 _location null
            (:`then`
              (`self.K2_DestroyActor` (`self.UnitGhost`)))))))))

(event `EnhancedInput|/Game/DIOURI/Input/IA_ND_LeftMouseClick`
  (params (ActionValue :type Boolean) (ElapsedSeconds :type "Float (double-precision)") (TriggeredSeconds :type "Float (double-precision)") (InputAction :type "InputAction Object Reference" :default "/Game/DIOURI/Input/IA_ND_LeftMouseClick.IA_ND_LeftMouseClick"))
  (bind (_locationx _locationy) (`self.GetMousePosition`))
  (bind _bp_hud (`self.BP HUD`))
  ;[0.1875 0.1875 0.1875] Left Click
  (:`Started`
    (if (`self.IsEventing`)
      (`/Game/DIOURI/BP_AOEDamageEvent.Quit Selecting` (`self.eventCylinder`))
      (set `self.IsEventing` false)
      (`self.K2_DestroyActor` (`self.eventCylinder`))
      (else
        (set `/Game/DIOURI/BP_ND_HUD.InitMousePos` (`KismetMathLibrary.MakeVector2D` _locationx _locationy) _bp_hud)
        (set `/Game/DIOURI/BP_ND_HUD.IsDrawing` true _bp_hud)
        (bind _selected_dumy (`self.selected dumy`)
          (:`then`
            (`/Game/DIOURI/Unit/BP_ND_Dumy.SetSelected` _selected_dumy false)
            (set `self.selected dumy` null))
          (:`else`
            _))
        (`KismetSystemLibrary.PrintString` "click")
        (bind _asbp_nd_dumy (cast `/Game/DIOURI/Unit/BP_ND_Dumy` (`.HitActor` (`GameplayStatics.BreakHitResult` (`self.GetHitResultUnderCursorByChannel` "TraceTypeQuery1")))))
        (`/Game/DIOURI/Unit/BP_ND_Dumy.SetSelected` _asbp_nd_dumy true)
        (set `self.selected dumy` _asbp_nd_dumy))))
  (:`Canceled`
    (set `/Game/DIOURI/BP_ND_HUD.IsDrawing` false (`self.BP HUD`) :!label _label))
  (:`Completed`
    (goto _label)))

(event `self.ReceiveTick`
  (params (DeltaSeconds :type "Float (single-precision)"))
  (bind _returnvalue_x (`KismetMathLibrary.BreakVector2D` (`WidgetLayoutLibrary.GetViewportSize`)))
  (bind _returnvalue_x_2 (`KismetMathLibrary.BreakVector2D` (`WidgetLayoutLibrary.GetViewportSize`)))
  (bind (_returnvalue_x_3 _returnvalue_y) (`KismetMathLibrary.BreakVector2D` (`WidgetLayoutLibrary.GetViewportSize`)))
  (bind (_returnvalue_x_4 _returnvalue_y_2) (`KismetMathLibrary.BreakVector2D` (`WidgetLayoutLibrary.GetViewportSize`)))
  (bind _output_get (set `self.CameraBorderMovementVector` (0.0 0.0 0.0)))
  (if (<= (`.LocationY` (`self.GetMousePosition`)) (* _returnvalue_y (`self.VerticalBorderDeadZone`)))
    (bind _output_get_2 (set `self.CameraBorderMovementVector` (+ _output_get (0.0 1.0 0.0)))))
  (if (>= (`.LocationY` (`self.GetMousePosition`)) (- _returnvalue_y_2 (* _returnvalue_y_2 (`self.VerticalBorderDeadZone`))))
    (bind _output_get_3 (set `self.CameraBorderMovementVector` (+ _output_get_2 (0.0 -1.0 0.0)))))
  (if (<= (`self.GetMousePosition`) (* _returnvalue_x_2 (`self.Horizontal Border Dead Zone`)))
    (bind _output_get_4 (set `self.CameraBorderMovementVector` (+ _output_get_3 (-1.0 0.0 0.0)))))
  (if (>= (`self.GetMousePosition`) (- _returnvalue_x (* _returnvalue_x (`self.Horizontal Border Dead Zone`))))
    (bind _output_get_5 (set `self.CameraBorderMovementVector` (+ _output_get_4 (1.0 0.0 0.0)))))
  (`EnhancedInputSubsystemInterface.InjectInputVectorForAction` :`self` (subsystem `EnhancedInputLocalPlayerSubsystem`) :`Action` "/Game/DIOURI/Input/IA_ND_CameraMove.IA_ND_CameraMove" :`Value` _output_get_5))

(event `Key|B`
  (params (Key :type "Key Structure"))
  (:`Pressed`
    (if (not (`self.IsEventing`))
      (bind _returnvalue (`|SpawnActorFromClass` "/Game/DIOURI/BP_AOEDamageEvent.BP_AOEDamageEvent_C" (`KismetMathLibrary.MakeTransform` (0.0 0.0 0.0)) "Undefined" "MultiplyWithRoot" null null))
      (bind _output_get (set `self.eventCylinder` _returnvalue))
      (`/Game/DIOURI/BP_AOEDamageEvent.Select area` _output_get)
      (set `self.IsEventing` true))))

(fn `Get location Under Cursor`
  (returns (Hit :type Boolean) (Location :type "Vector Structure"))
  (bind (_bblockinghit _binitialoverlap _time _distance _location) (`GameplayStatics.BreakHitResult` (`self.GetHitResultUnderCursorByChannel` "TraceTypeQuery1")))
  (return _bblockinghit _location))

(fn `UserConstructionScript`)