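; AOE damage event actor that lets its DamageZone follow the mouse cursor for area selection; it contains no damage logic.
; Selectarea and QuitSelecting switch the FollowMouse flag on and off.
; While it is on, Tick line-traces from the deprojected cursor on the Visibility channel and moves DamageZone to the hit location.
; That world-space location is applied as a relative location, without checking for a hit.
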(event `Select area`
  (set `self.FollowMouse` true))

(event `Quit Selecting`
  (set `self.FollowMouse` false))

(event `self.ReceiveTick`
  (params (DeltaSeconds :type "Float (single-precision)"))
  (bind (_worldlocation _worlddirection) (`PlayerController.DeprojectMousePositionToWorld` (`GameplayStatics.GetPlayerController` 0)))
  (if (`self.FollowMouse`)
    (bind _outhit (`KismetSystemLibrary.LineTraceSingle` _worldlocation (+ _worldlocation (* _worlddirection 100000.0)) "TraceTypeQuery1"))
    (`SceneComponent.K2_SetRelativeLocation` (`self.DamageZone`) (`KismetMathLibrary.MakeVector` (.x (`.Location` (`GameplayStatics.BreakHitResult` _outhit))) (.y (`.Location` (`GameplayStatics.BreakHitResult` _outhit))) (.z (`.Location` (`GameplayStatics.BreakHitResult` _outhit)))) false false)))

(fn `UserConstructionScript`)