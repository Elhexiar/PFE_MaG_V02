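; BPC_RessourcesBar is a resource bar Blueprint that passively refills two values, PRessources and TRessource, over time.
; While their combined total is below 1.0, Tick accumulates a separate timer for each and adds a fixed increment to that resource every second.
; Once the total reaches the cap, both timers reset; the values themselves are not clamped.
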(event `self.ReceiveTick`
  (params (DeltaSeconds :type "Float (single-precision)"))
  (if (< (+ (`self.P_Ressources`) (`self.T_Ressource`)) 1.0)
    (set `self.P_Time` (+ DeltaSeconds (`self.P_Time`)))
    (set `self.T_Time` (+ DeltaSeconds (`self.T_Time`)))
    (`|ExecutionSequence`
      (:`then_0`
        (if (>= (`self.P_Time`) 1.0)
          (set `self.P_Time` 0.0)
          (set `self.P_Ressources` (+ (`self.P_Ressources`) 0.1))))
      (:`then_1`
        (if (>= (`self.T_Time`) 1.0)
          (set `self.T_Time` 0.0)
          (set `self.T_Ressource` (+ (`self.T_Ressource`) 0.1)))))
    (else
      (set `self.P_Time` 0.0)
      (set `self.T_Time` 0.0))))