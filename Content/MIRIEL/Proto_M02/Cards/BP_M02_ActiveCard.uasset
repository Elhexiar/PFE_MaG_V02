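; BP_M02_ActiveCard is a card Blueprint in the M02 prototype, with play, draw, discard, move and swap hooks.
; OnPlay takes its success from CheckCost and never flags the card for destruction.
; CheckCost compares Cost with the player resource manager's current resources and prints a debug message when affordable, without spending any.
; Both CheckCost branches return false, so playing always fails; the other hooks are empty.
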(fn `CheckCost`
  (returns (CostCheckSuccess :type Boolean))
  (bind _bpc_playerressourcemanager (`/Game/MIRIEL/Proto_M02/Player/BP_M02_RTSControler.BPC_PlayerRessourceManager` (`self.PlayerController`)))
  (bind _currentressources (`/Game/MIRIEL/Proto_M02/Player/BPC_PlayerRessourceManager.CurrentRessources` _bpc_playerressourcemanager))
  (if (>= (- _currentressources (`self.Cost`)) 0)
    (`KismetSystemLibrary.PrintString` _bpc_playerressourcemanager (`KismetStringLibrary.Concat_StrStr` "you have enough ressources it costs  : " (`KismetStringLibrary.Conv_IntToString` (`self.Cost`)) " and you have : " (`KismetStringLibrary.Conv_IntToString` _currentressources) "/" (`KismetStringLibrary.Conv_IntToString` (`/Game/MIRIEL/Proto_M02/Player/BPC_PlayerRessourceManager.MaxRessources` _bpc_playerressourcemanager))))
    (return false)
    (else
      (return false))))

(fn `OnDiscard`)

(fn `OnDraw`)

(fn `OnMove`)

(fn `OnPlay`
  (returns (Success :type Boolean) (ShouldDestroyCardAfter :type Boolean))
  (bind _costchecksuccess (`self.CheckCost`))
  (if _costchecksuccess
    (return true false)
    (else
      (return false false))))

(fn `OnSwap`)