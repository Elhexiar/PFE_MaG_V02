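; Card actor in the player's hand for the M02 prototype, reacting to being moved along the hand or toward spawning.
; While moving, Tick checks its relative Y against neighbouring holders to request swaps from the player hand manager.
; Crossing an X threshold toggles spawn mode, fading body materials and widget background.
; DestroyCard clears its holder, has the manager reorganise the hand, and removes the card from its lists.
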(event `self.ReceiveBeginPlay`
  (bind _asbp_m02_rtscontroler (`/Game/MIRIEL/Proto_M02/Utils/BPFL_M02_Utils.Get_M02_PlayerController`))
  (set `self.BPC M02 Player Hand Manager` (`/Game/MIRIEL/Proto_M02/Player/BP_M02_RTSControler.BPC_M02_PlayerHandManager` _asbp_m02_rtscontroler))
  (bind _returnvalue (`MaterialInterface.GetBaseMaterial` (`PrimitiveComponent.GetMaterial` (`self.CardBody`) 0)))
  (set `self.InitialMaterial0` _returnvalue)
  (bind _returnvalue_2 (`MaterialInterface.GetBaseMaterial` (`PrimitiveComponent.GetMaterial` (`self.CardBody`) 1)))
  (set `self.InitialMaterial1` _returnvalue_2)
  (bind _returnvalue_3 (`MaterialInterface.GetBaseMaterial` (`PrimitiveComponent.GetMaterial` (`self.CardBody`) 1)))
  (set `self.InitialMaterial2` _returnvalue_3))

(event `self.ReceiveTick`
  (params (DeltaSeconds :type "Float (single-precision)"))
  (if (`self.isMoving`)
    (`self.RightSideCheckForSwap`)
    (`self.LeftSideCheckForSwap`)
    (`self.CheckForSpawnMode`)))

(fn `CheckForSpawnMode`
  (if (<= (.x (.location (`SceneComponent.GetRelativeTransform` (`self.DefaultSceneRoot`)))) (`self.SpawnThreshold`))
    (if (not (`self.SpawningMode`))
      (set `self.SpawningMode` true)
      (`self.SetMaterialToTransparent`))
    (elif (`self.SpawningMode`)
      (set `self.SpawningMode` false)
      (`self.SetMaterialToDefault`))))

(fn `DestroyCard`
  (`/Game/MIRIEL/Proto_M02/Cards/InHand/BP_M02_CardHolder.ClearHoldedCard` (`self.Holder`))
  (set `self.Holder` null)
  (bind _asbp_m02_rtscontroler (`/Game/MIRIEL/Proto_M02/Utils/BPFL_M02_Utils.Get_M02_PlayerController`))
  (bind _bpc_m02_playerhandmanager (`/Game/MIRIEL/Proto_M02/Player/BP_M02_RTSControler.BPC_M02_PlayerHandManager` _asbp_m02_rtscontroler))
  (`/Game/MIRIEL/Proto_M02/Player/BPC_M02_PlayerHandManager.Reorganise Hand Once V3` _bpc_m02_playerhandmanager)
  (`KismetArrayLibrary.Array_RemoveItem` (`/Game/MIRIEL/Proto_M02/Player/BPC_M02_PlayerHandManager.PlayerCardList` _bpc_m02_playerhandmanager) (`self.Card`))
  (bind _returnvalue (`KismetArrayLibrary.Array_RemoveItem` (`/Game/MIRIEL/Proto_M02/Player/BPC_M02_PlayerHandManager.InHandCardActorList` _bpc_m02_playerhandmanager) self))
  (if _returnvalue
    (`self.K2_DestroyActor`)
    (else
      (`KismetSystemLibrary.PrintString` "Bizzare"))))

(fn `LeftSideCheckForSwap`
  (if (!= (`/Game/MIRIEL/Proto_M02/Cards/InHand/BP_M02_CardHolder.InitialLeftSideHolderIndex` (`self.Holder`)) -1)
    (if (`KismetSystemLibrary.IsValid` (`/Game/MIRIEL/Proto_M02/Cards/InHand/BP_M02_CardHolder.InHandCardRef` (`/Game/MIRIEL/Proto_M02/Cards/InHand/BP_M02_CardHolder.LeftSideHolder` (`self.Holder`))))
      (if (>= (.y (.location (`SceneComponent.GetRelativeTransform` (`self.DefaultSceneRoot`)))) (`/Game/MIRIEL/Proto_M02/Cards/InHand/BP_M02_CardHolder.DistanceToLeftHolder` (`self.Holder`)))
        (`KismetSystemLibrary.PrintString` "Left Swap")
        (`/Game/MIRIEL/Proto_M02/Player/BPC_M02_PlayerHandManager.Immediate Swap Between Valid Cards` (`self.BPC M02 Player Hand Manager`) (`self.Holder`) (`/Game/MIRIEL/Proto_M02/Cards/InHand/BP_M02_CardHolder.LeftSideHolder` (`self.Holder`)))))))

(fn `RightSideCheckForSwap`
  (if (!= (`/Game/MIRIEL/Proto_M02/Cards/InHand/BP_M02_CardHolder.InitialRightSideHolderIndex` (`self.Holder`)) -1)
    (if (`KismetSystemLibrary.IsValid` (`/Game/MIRIEL/Proto_M02/Cards/InHand/BP_M02_CardHolder.InHandCardRef` (`/Game/MIRIEL/Proto_M02/Cards/InHand/BP_M02_CardHolder.RightSideHolder` (`self.Holder`))))
      (if (<= (.y (.location (`SceneComponent.GetRelativeTransform` (`self.DefaultSceneRoot`)))) (`/Game/MIRIEL/Proto_M02/Cards/InHand/BP_M02_CardHolder.DistanceToRightHolder` (`self.Holder`)))
        (`KismetSystemLibrary.PrintString` "Right Swap")
        (`/Game/MIRIEL/Proto_M02/Player/BPC_M02_PlayerHandManager.Immediate Swap Between Valid Cards` (`self.BPC M02 Player Hand Manager`) (`self.Holder`) (`/Game/MIRIEL/Proto_M02/Cards/InHand/BP_M02_CardHolder.RightSideHolder` (`self.Holder`)))))))

(fn `SetMaterialToDefault`
  (`PrimitiveComponent.SetMaterial` (`self.CardBody`) 0 (`self.InitialMaterial0`))
  (`PrimitiveComponent.SetMaterial` (`self.CardBody`) 1 (`self.InitialMaterial1`))
  (`PrimitiveComponent.SetMaterial` (`self.CardBody`) 2 (`self.InitialMaterial2`))
  (bind _aswbp_in_hand_card_widget (cast `/Game/MIRIEL/Proto_M02/Cards/InHand/WBP_InHandCardWidget` (`WidgetComponent.GetWidget` (`self.CardWidget`))))
  (bind _backgroundimage (`/Game/MIRIEL/Proto_M02/Cards/InHand/WBP_InHandCardWidget.BackgroundImage` _aswbp_in_hand_card_widget))
  (bind (_colorandopacity_r _colorandopacity_g _colorandopacity_b) (break `LinearColor` (`Image.ColorAndOpacity` _backgroundimage)))
  (set `Image.ColorAndOpacity` (make `LinearColor` _colorandopacity_r _colorandopacity_g _colorandopacity_b 1.0) _backgroundimage))

(fn `SetMaterialToTransparent`
  (`PrimitiveComponent.SetMaterial` (`self.CardBody`) 0 "/Game/MIRIEL/Proto_M02/Utils/M_M02_TranslusentTestMaterial.M_M02_TranslusentTestMaterial")
  (`PrimitiveComponent.SetMaterial` (`self.CardBody`) 1 "/Game/MIRIEL/Proto_M02/Utils/M_M02_TranslusentTestMaterial.M_M02_TranslusentTestMaterial")
  (`PrimitiveComponent.SetMaterial` (`self.CardBody`) 2 "/Game/MIRIEL/Proto_M02/Utils/M_M02_TranslusentTestMaterial.M_M02_TranslusentTestMaterial")
  (bind _aswbp_in_hand_card_widget (cast `/Game/MIRIEL/Proto_M02/Cards/InHand/WBP_InHandCardWidget` (`WidgetComponent.GetWidget` (`self.CardWidget`))))
  (bind _backgroundimage (`/Game/MIRIEL/Proto_M02/Cards/InHand/WBP_InHandCardWidget.BackgroundImage` _aswbp_in_hand_card_widget))
  (bind (_colorandopacity_r _colorandopacity_g _colorandopacity_b) (break `LinearColor` (`Image.ColorAndOpacity` _backgroundimage)))
  (set `Image.ColorAndOpacity` (make `LinearColor` _colorandopacity_r _colorandopacity_g _colorandopacity_b 0.2) _backgroundimage))

(fn `UserConstructionScript`)