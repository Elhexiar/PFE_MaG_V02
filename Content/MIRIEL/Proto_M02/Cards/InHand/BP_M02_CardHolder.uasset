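; BP_M02_CardHolder is a slot actor in the player's hand of cards, holding a reference to an in-hand card that can be cleared.
; On BeginPlay it gets the M02 player controller and looks up its left and right neighbor holders by index in the hand manager's CardHolderMap, skipping unset indices.
; It caches the distance to each neighbor, negating the right-side value.
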(event `self.ReceiveBeginPlay`
  (bind _initialleftsideholderindex (`self.InitialLeftSideHolderIndex`))
  (bind _initialrightsideholderindex (`self.InitialRightSideHolderIndex`))
  (bind _asbp_m02_rtscontroler (`/Game/MIRIEL/Proto_M02/Utils/BPFL_M02_Utils.Get_M02_PlayerController`))
  (bind _output_get (set `self.BP M02 RTSControler` _asbp_m02_rtscontroler))
  (if (!= _initialleftsideholderindex -1)
    (bind _cardholdermap (`/Game/MIRIEL/Proto_M02/Player/BPC_M02_PlayerHandManager.CardHolderMap` (`/Game/MIRIEL/Proto_M02/Player/BP_M02_RTSControler.BPC_M02_PlayerHandManager` _output_get)))
    (bind _output_get_2 (set `self.LeftSideHolder` (`BlueprintMapLibrary.Map_Find` _cardholdermap _initialleftsideholderindex)))
    (set `self.DistanceToLeftHolder` (`KismetMathLibrary.Vector_Distance` (`self.K2_GetActorLocation` self) (`self.K2_GetActorLocation` _output_get_2))))
  (if (!= _initialrightsideholderindex -1)
    (bind _output_get_3 (set `self.RightSideHolder` (`BlueprintMapLibrary.Map_Find` _cardholdermap _initialrightsideholderindex)))
    (set `self.DistanceToRightHolder` (* (`KismetMathLibrary.Vector_Distance` (`self.K2_GetActorLocation` self) (`self.K2_GetActorLocation` _output_get_3)) -1.0))))

(fn `ClearHoldedCard`
  (set `self.InHandCardRef` null))

(fn `UserConstructionScript`)