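; BP_M02_CardHolderPanel is an actor that groups four card holder slots, apparently for in-hand cards in the M02 prototype.
; Its construction script casts the child actors of four ChildActor components to BP_M02_CardHolder and stores them as Holder0 to Holder3 references.
; Each cast runs in sequence, so a failed one leaves the remaining references unset; the event graph holds no active logic.
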(fn `UserConstructionScript`
  (locals (Holder0 :type "/Game/MIRIEL/Proto_M02/Cards/InHand/BP_M02_CardHolder Object Reference") (Holder1 :type "/Game/MIRIEL/Proto_M02/Cards/InHand/BP_M02_CardHolder Object Reference") (Holder2 :type "/Game/MIRIEL/Proto_M02/Cards/InHand/BP_M02_CardHolder Object Reference") (Holder3 :type "/Game/MIRIEL/Proto_M02/Cards/InHand/BP_M02_CardHolder Object Reference"))
  (bind _asbp_m02_card_holder (cast `/Game/MIRIEL/Proto_M02/Cards/InHand/BP_M02_CardHolder` (`ChildActorComponent.ChildActor` (`self.CardHolder_00`))))
  (set `local.Holder0` _asbp_m02_card_holder)
  (bind _asbp_m02_card_holder_2 (cast `/Game/MIRIEL/Proto_M02/Cards/InHand/BP_M02_CardHolder` (`ChildActorComponent.ChildActor` (`self.CardHolder_01`))))
  (set `local.Holder1` _asbp_m02_card_holder_2)
  (bind _asbp_m02_card_holder_3 (cast `/Game/MIRIEL/Proto_M02/Cards/InHand/BP_M02_CardHolder` (`ChildActorComponent.ChildActor` (`self.CardHolder_02`))))
  (set `local.Holder2` _asbp_m02_card_holder_3)
  (bind _asbp_m02_card_holder_4 (cast `/Game/MIRIEL/Proto_M02/Cards/InHand/BP_M02_CardHolder` (`ChildActorComponent.ChildActor` (`self.CardHolder_03`))))
  (set `local.Holder3` _asbp_m02_card_holder_4))