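; Temporary prototype card that deals area damage at the point under the cursor when played.
; OnPlay runs the parent check, traces under the cursor, spends the cost, spawns VFX and sphere-traces for squad units to damage through their stat components.
; It reports success and card destruction only when a squad is found, though cost and VFX apply on any ground hit.
; OnMove only calls its parent.
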(fn `OnMove`
  (`parent.OnMove`))

(fn `OnPlay`
  (returns (Success :type Boolean) (ShouldDestroyCardAfter :type Boolean))
  (bind _playercontroller (`self.PlayerController`))
  (bind _hitresult (`PlayerController.GetHitResultUnderCursorByChannel` (`self.PlayerController`) "TraceTypeQuery4" false))
  (bind _bpc_playerressourcemanager (`/Game/MIRIEL/Proto_M02/Player/BP_M02_RTSControler.BPC_PlayerRessourceManager` _playercontroller))
  (bind _success (`parent.OnPlay`))
  (if _success
    (if (`GameplayStatics.BreakHitResult` _hitresult)
      (set `self.LocationToCheck` (`.Location` (`GameplayStatics.BreakHitResult` _hitresult)))
      (`KismetSystemLibrary.PrintString` null "BOOM")
      (`/Game/MIRIEL/Proto_M02/Player/BPC_PlayerRessourceManager.RemoveRessource` (`/Game/MIRIEL/Proto_M02/Player/BP_M02_RTSControler.BPC_PlayerRessourceManager` (`self.PlayerController`)) (`self.Cost`))
      (`/Game/MIRIEL/Proto_M02/Player/BP_M02_RTSControler.SpawnVFXSystem` :`self` (`self.PlayerController`) :`SystemTemplate` (`self.VFXClass`) :`Location` (`self.LocationToCheck`) :`Scale` (1.0 1.0 1.0) :`bAutoDestroy` true :`bAutoActivate` true)
      (bind (_unitlist1 _squadlist1 _foundsquad) (`/Game/MIRIEL/Proto_M02/Player/BP_M02_RTSControler.DetectSquadFromSphereTrace` (`self.PlayerController`) (`self.LocationToCheck`) (`self.Radius`)))
      (if _foundsquad
        (for _array_element _unitlist1
          (`/Game/MIRIEL/Proto_M02/Unit/Old/M02_BPC_UnitStatComponent.TakeDamage` (`/Game/MIRIEL/Proto_M02/Unit/Old/BP_M02_SelectableUnit_deprecated.UnitStatComponent` _array_element) (`self.Damage`)))
        (return true true)
        (else
          (`KismetSystemLibrary.PrintString` null "NoUnitFound")))
      (else
        (`KismetSystemLibrary.PrintString` null "could not hit under cursor")))
    (else
      (`KismetSystemLibrary.PrintString` _playercontroller (`KismetStringLibrary.Concat_StrStr` "Not enough Ressources :" (`KismetStringLibrary.Conv_IntToString` (`/Game/MIRIEL/Proto_M02/Player/BPC_PlayerRessourceManager.CurrentRessources` _bpc_playerressourcemanager)) "/" (`KismetStringLibrary.Conv_IntToString` (`/Game/MIRIEL/Proto_M02/Player/BPC_PlayerRessourceManager.MaxRessources` _bpc_playerressourcemanager)))))))