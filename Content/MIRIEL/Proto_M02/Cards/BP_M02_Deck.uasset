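; BP_M02_Deck is a card deck for the M02 prototype, storing its cards in CardList with index 0 as the top.
; PickTopCard removes and returns the top card with a not-empty flag, while add functions insert on top or at a random index.
; RemoveCard also removes only the top card, and Shuffle and PickRandomCard are empty stubs.
; A debug function returns a random card without removing it.
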(fn `AddCardAtRandomIndex`
  (params (cardToAdd :type "Card Object Reference"))
  (bind _cardlist (`self.cardList`))
  (`KismetArrayLibrary.Array_Insert` _cardlist cardToAdd (`KismetMathLibrary.RandomIntegerInRange` 0 (`KismetArrayLibrary.Array_Length` _cardlist))))

(fn `AddTopCard`
  (params (NewCard :type "Card Object Reference"))
  (`KismetArrayLibrary.Array_Insert` (`self.cardList`) NewCard))

(fn `DebugPickDuplicateRandomCard`
  (returns (Card :type "Card Object Reference"))
  (bind _cardlist (`self.cardList`))
  (return (`|GetArrayItem` _cardlist (`.OutIndex` (`KismetArrayLibrary.Array_Random` _cardlist)))))

(fn `Pick Top Card`
  (returns (PickedCard :type "Card Object Reference") (isNotEmpty :type Boolean))
  (locals (TopCardPicked :type "Card Object Reference") (NotEmptyStatus :type Boolean :default true))
  (bind _cardlist (`self.cardList`))
  (if (`KismetArrayLibrary.Array_IsNotEmpty` _cardlist)
    (set `local.TopCardPicked` (`|GetArrayItem` _cardlist))
    (`self.RemoveTopCard`)
    (return (`local.TopCardPicked`) true)
    (else
      (return null false))))

(fn `PickRandomCard`
  (returns (PickedCard :type "Card Object Reference"))
  (return null))

(fn `RemoveCard`
  (`KismetArrayLibrary.Array_Remove` (`self.cardList`)))

(fn `RemoveTopCard`
  (`KismetArrayLibrary.Array_Remove` (`self.cardList`)))

(fn `Shuffle`)