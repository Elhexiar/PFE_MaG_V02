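; Temporary prototype card that gives a speed buff to a squad on team 0 picked under the cursor.
; On play, after the parent check passes, it traces to a deprecated selectable unit and adds a new timed speed hediff to each unit in that squad.
; Success deducts the resource cost and flags the card for destruction; a failed parent check prints a not-enough-resources message.
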(fn `OnMove`
  (`parent.OnMove`))

(fn `OnPlay`
  (returns (Success :type Boolean) (ShouldDestroyCardAfter :type Boolean))
  (bind _playercontroller (`self.PlayerController`))
  (bind _bpc_playerressourcemanager (`/Game/MIRIEL/Proto_M02/Player/BP_M02_RTSControler.BPC_PlayerRessourceManager` _playercontroller))
  (bind _success (`parent.OnPlay`))
  (if _success
    (bind _asbp_m02_selectable_unit_deprecated (cast `/Game/MIRIEL/Proto_M02/Unit/Old/BP_M02_SelectableUnit_deprecated` (`.HitActor` (`GameplayStatics.BreakHitResult` (`PlayerController.GetHitResultUnderCursorByChannel` (`self.PlayerController`) "TraceTypeQuery4" false))))
      (:`then`
        (bind _parentsquad (`/Game/MIRIEL/Proto_M02/Unit/Old/BP_M02_SelectableUnit_deprecated.ParentSquad` _asbp_m02_selectable_unit_deprecated))
        (if (== (`/Game/MIRIEL/Proto_M02/Unit/Squad/BP_M02_Squad_Default.TeamNumber` _parentsquad) 0)
          (for _array_element (`/Game/MIRIEL/Proto_M02/Unit/Squad/BP_M02_Squad_Default.UnitList` _parentsquad)
            (bind _returnvalue (`|GenericCreateObject` "/Game/MIRIEL/Proto_M02/Unit/Hedif/HedifObjects/BP_M02_SpeedBuff.BP_M02_SpeedBuff_C" (`self.SpeedBuffAmount`) _array_element (`self.Duration`)))
            (`/Game/MIRIEL/Proto_M02/Unit/Old/BPC_M02_UnitHedifComponent.AddNewHediff` (`/Game/MIRIEL/Proto_M02/Unit/Old/BP_M02_SelectableUnit_deprecated.BPC_M02_UnitHedifComponent` _array_element) _returnvalue))
          (`/Game/MIRIEL/Proto_M02/Player/BPC_PlayerRessourceManager.RemoveRessource` (`/Game/MIRIEL/Proto_M02/Player/BP_M02_RTSControler.BPC_PlayerRessourceManager` (`self.PlayerController`)) (`self.Cost`))
          (return true true)
          (else
            _)))
      (:`CastFailed`
        _))
    (return false false)
    (else
      (`KismetSystemLibrary.PrintString` _playercontroller (`KismetStringLibrary.Concat_StrStr` "Not enough Ressources :" (`KismetStringLibrary.Conv_IntToString` (`/Game/MIRIEL/Proto_M02/Player/BPC_PlayerRessourceManager.CurrentRessources` _bpc_playerressourcemanager)) "/" (`KismetStringLibrary.Conv_IntToString` (`/Game/MIRIEL/Proto_M02/Player/BPC_PlayerRessourceManager.MaxRessources` _bpc_playerressourcemanager))))
      (return false false))))