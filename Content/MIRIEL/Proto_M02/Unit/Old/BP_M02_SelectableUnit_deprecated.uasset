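; Deprecated selectable squad unit for the M02 prototype that carries out move commands and handles its own death.
; MoveTo stores the handler, runs AIMoveTo, and on success clears IsMoving and pops the command from its command stack component.
; While moving, Tick updates Origin and optionally draws velocity and destination debug lines.
; Die removes the unit and handler from ParentSquad, then destroys both; construction links the stat component to the unit.
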(event `Move To`
  (params (Location :type "Vector Structure") (Command :type "/Game/MIRIEL/Proto_M02/Unit/UnitCommands/BP_M02_MoveCommand Object Reference") (Handler :type "/Game/MIRIEL/Proto_M02/Unit/Squad/BP_M02_Handler Object Reference"))
  (set `self.CurrentHandler` Handler)
  (`|AIMoveTo` self Location null
    (:`then`
      (set `self.Destination` Location)
      (set `self.Origin` (`self.K2_GetActorLocation`))
      (set `self.Is Moving` true))
    (:`OnSuccess`
      (set `self.Is Moving` false)
      (`/Game/MIRIEL/Proto_M02/Utils/BPFL_M02_Utils.Get_M02_PlayerController`)
      (`/Game/MIRIEL/Proto_M02/Unit/UnitCommands/BPC_UnitCommandStack.Pop Command by Object` (`self.BPC_UnitCommandStack`) Command))))

(event `self.ReceiveTick`
  (params (DeltaSeconds :type "Float (single-precision)"))
  (if (`self.Is Moving`)
    (bind _output_get (set `self.Origin` (`self.K2_GetActorLocation`)))
    (if (`self.drawDebugMovementLine`)
      (`KismetSystemLibrary.DrawDebugLine` _output_get (+ _output_get (`self.GetVelocity`)) (struct :`G` 0.149541 :`B` 1.0 :`A` 1.0) 0.1 5.0)
      (`KismetSystemLibrary.DrawDebugLine` (`self.Origin`) (`self.Destination`) (struct :`G` 1.0 :`B` 0.016063 :`A` 1.0) 0.1 2.0))))

(event `Die`
  (bind _parentsquad (`self.ParentSquad`))
  (bind _currenthandler (`self.CurrentHandler`))
  (`KismetArrayLibrary.Array_RemoveItem` (`/Game/MIRIEL/Proto_M02/Unit/Squad/BP_M02_Squad_Default.UnitList` _parentsquad) self)
  (`KismetArrayLibrary.Array_RemoveItem` (`/Game/MIRIEL/Proto_M02/Unit/Squad/BP_M02_Squad_Default.HandlerList` _parentsquad) _currenthandler)
  (`/Game/MIRIEL/Proto_M02/Unit/Squad/BP_M02_Handler.DestroyHandler` _currenthandler)
  (`self.K2_DestroyActor`))

(event `self.Range0.OnComponentBeginOverlap`
  (params (OverlappedComponent :type "PrimitiveComponent Object Reference") (OtherActor :type "Actor Object Reference") (OtherComp :type "PrimitiveComponent Object Reference") (OtherBodyIndex :type Integer) (bFromSweep :type Boolean) (SweepResult :type "HitResult Structure (by ref)")))

(event `self.Range0.OnComponentEndOverlap`
  (params (OverlappedComponent :type "PrimitiveComponent Object Reference") (OtherActor :type "Actor Object Reference") (OtherComp :type "PrimitiveComponent Object Reference") (OtherBodyIndex :type Integer)))

(fn `UserConstructionScript`
  (set `/Game/MIRIEL/Proto_M02/Unit/Old/M02_BPC_UnitStatComponent.ParentUnit` self (`self.UnitStatComponent`)))