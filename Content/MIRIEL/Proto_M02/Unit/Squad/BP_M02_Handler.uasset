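; BP_M02_Handler is a prototype squad handler actor that turns its static mesh position into ground destinations for the unit it handles.
; MoveUnit traces 5000 units straight down on Visibility, then pushes a new BP_M02_MoveCommand for the hit location onto the unit's command stack.
; SendTargetedCoordinates returns the hit from a similar trace on a different channel.
; Both traces draw debug circles, and DestroyHandler logs before destroying the actor.
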(fn `DestroyHandler`
  (`KismetSystemLibrary.PrintString` (`KismetStringLibrary.Concat_StrStr` "destroying " (`KismetSystemLibrary.GetDisplayName` self)))
  (`self.K2_DestroyActor`))

(fn `Move Unit`
  (bind _unittohandle (`self.UnitToHandle`))
  (bind _returnvalue (`SceneComponent.K2_GetComponentLocation` (`self.StaticMesh`)))
  (bind _outhit (`KismetSystemLibrary.LineTraceSingle` _returnvalue (- _returnvalue (0.0 0.0 5000.0)) "TraceTypeQuery1"))
  (bind (_bblockinghit _binitialoverlap _time _distance _location) (`GameplayStatics.BreakHitResult` _outhit))
  (`KismetSystemLibrary.DrawDebugCircle` _location 40.0 12 (struct :`R` 1.0 :`G` 0.115883 :`A` 1.0) 0.5 15.0 (1.0 0.0 0.0) (0.0 1.0 0.0))
  (bind _returnvalue_2 (`|GenericCreateObject` "/Game/MIRIEL/Proto_M02/Unit/UnitCommands/BP_M02_MoveCommand.BP_M02_MoveCommand_C" _location self _unittohandle))
  (`/Game/MIRIEL/Proto_M02/Unit/UnitCommands/BPC_UnitCommandStack.Add New Command` (`/Game/MIRIEL/Proto_M02/Unit/Old/BP_M02_SelectableUnit_deprecated.BPC_UnitCommandStack` _unittohandle) _returnvalue_2 0))

(fn `SendTargetedCoordinates`
  (returns (Location :type "Vector Structure"))
  (bind _returnvalue (`SceneComponent.K2_GetComponentLocation` (`self.StaticMesh`)))
  (bind _outhit (`KismetSystemLibrary.LineTraceSingle` _returnvalue (- _returnvalue (0.0 0.0 5000.0)) "TraceTypeQuery4"))
  (bind (_bblockinghit _binitialoverlap _time _distance _location) (`GameplayStatics.BreakHitResult` _outhit))
  (`KismetSystemLibrary.DrawDebugCircle` _location 40.0 12 (struct :`R` 1.0 :`B` 0.843322 :`A` 1.0) 0.5 15.0 (1.0 0.0 0.0) (0.0 1.0 0.0))
  (return _location))

(fn `UserConstructionScript`)