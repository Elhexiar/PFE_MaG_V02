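; Squad actor that spawns a grid formation of units from a formation data asset, each paired with an attached handler marking its slot.
; Move events trigger the handlers, with V2 first clearing unit commands and refreshing each handler's target.
; V2 then reassigns greedily: units farthest from the squad's ground point, traced at BeginPlay, claim the nearest type-compatible handler first.
; Selection toggles every unit's marker.
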(event Custom|Move%20All%20Units%20V1
  (for _array_element (Variables|Default|GetHandlerList)
    (Default|MoveUnit _array_element)))

(event Custom|Move%20All%20Unit%20V2
  ;[1 1 1] Clear Handler
  (for _array_element (Variables|Default|GetHandlerList)
    (Default|ClearCommandList (Variables|/Game/MIRIEL/Proto_M02/Unit/Old/BP_M02_SelectableUnit_deprecated.BP_M02_SelectableUnit_deprecated_C|GetBPC_UnitCommandStack (Variables|/Game/MIRIEL/Proto_M02/Unit/Squad/SquadSingleUnitHandler.SquadSingleUnitHandler_C|GetUnitToHandle _array_element)))
    (Variables|/Game/MIRIEL/Proto_M02/Unit/Squad/SquadSingleUnitHandler.SquadSingleUnitHandler_C|SetUnitToHandle _array_element 0)
    (bind _location (Default|SendTargetedCoordinates _array_element))
    (Variables|/Game/MIRIEL/Proto_M02/Unit/Squad/SquadSingleUnitHandler.SquadSingleUnitHandler_C|SetCurrentLocationToGoTo _array_element _location))
  (CallFunction|Reassign)
  (for _array_element_2 (Variables|Default|GetHandlerList)
    (Default|MoveUnit _array_element_2)))

(event EventBeginPlay
  (bind _self self)
  (bind _self_2 self)
  (bind _spacinglength (Variables|Default|GetSpacingLength))
  (bind _formationlength (Variables|Default|GetFormationLength))
  (bind _returnvalue (Math|Conversions|ToFloat(Integer) _formationlength))
  (bind _defaultsceneroot (Variables|Default|GetDefaultSceneRoot _self_2))
  (bind _defaultsceneroot_2 (Variables|Default|GetDefaultSceneRoot _self))
  (bind _returnvalue_2 (Transformation|GetWorldLocation _defaultsceneroot))
  (bind _returnvalue_3 (Transformation|GetWorldLocation _defaultsceneroot_2))
  (|CallParentFunction)
  (bind _outhit (Collision|LineTraceByChannel "0, 0, 0" (- (Transformation|GetWorldLocation (Variables|Default|GetDefaultSceneRoot)) "0.000000,0.000000,5000.000000") "TraceTypeQuery1" false 0 "None"))
  (Variables|Default|SetCurrentProjectedLocation (.Location (Collision|BreakHitResult _outhit)))
  (for _index (range 0 (- (Variables|Default|GetFormationLength) -1))
    (for _index_2 (range 0 (- (Variables|Default|GetFormationLength) -1))
      (if (Utilities|IsValidClass (.Value (Utilities|Map|Find (Variables|Default|GetSquadFormation) (Math|Vector2D|MakeVector2D (Math|Conversions|ToFloat(Integer) _index_2) (Math|Conversions|ToFloat(Integer) _index)))))
        (Rendering|Debug|DrawDebugArrow (Math|Vector|MakeVector (.x _returnvalue_2) (.y _returnvalue_2) (.z _returnvalue_2)) (Math|Vector|MakeVector (|((xOrigin-(((fLength-1)*fUnit)/2))+(index*fUnit)) _returnvalue _spacinglength (Math|Conversions|ToFloat(Integer) _index) (.x _returnvalue_3)) (|((yOrigin+(((fLength-1)*fUnit)/2))-(index*fUnit)) _returnvalue _spacinglength (Math|Conversions|ToFloat(Integer) _index_2) (.y _returnvalue_3)) 5e+02) 1.0 "(R=0.310191,G=1.000000,B=0.282459,A=1.000000)" 1e+01 1.0)
        (bind _returnvalue_4 (Game|SpawnActorfromClass (.Value (Utilities|Map|Find (Variables|Default|GetSquadFormation) (Math|Vector2D|MakeVector2D (Math|Conversions|ToFloat(Integer) _index_2) (Math|Conversions|ToFloat(Integer) _index)))) (Math|Transform|MakeTransform (Math|Vector|MakeVector (|((xOrigin-(((fLength-1)*fUnit)/2))+(index*fUnit)) _returnvalue _spacinglength (Math|Conversions|ToFloat(Integer) _index) (.x _returnvalue_3)) (|((yOrigin+(((fLength-1)*fUnit)/2))-(index*fUnit)) _returnvalue _spacinglength (Math|Conversions|ToFloat(Integer) _index_2) (.y _returnvalue_3)) 5e+02) "0, 0, 0" "1.000000,1.000000,1.000000") "Undefined" "MultiplyWithRoot" 0 self 0))
        (Utilities|Array|Add (Variables|Default|GetUnitList) _returnvalue_4)
        (bind _returnvalue_5 (Game|SpawnActorfromClass "/Game/MIRIEL/Proto_M02/Unit/Squad/SquadSingleUnitHandler.SquadSingleUnitHandler_C" (Math|Transform|MakeTransform (Math|Vector|MakeVector (|((xOrigin-(((fLength-1)*fUnit)/2))+(index*fUnit)) _returnvalue _spacinglength (Math|Conversions|ToFloat(Integer) _index) (.x _returnvalue_3)) (|((yOrigin+(((fLength-1)*fUnit)/2))-(index*fUnit)) _returnvalue _spacinglength (Math|Conversions|ToFloat(Integer) _index_2) (.y _returnvalue_3)) (Variables|Default|GetHandlerHeight)) "0, 0, 0" "1.000000,1.000000,1.000000") "Undefined" "MultiplyWithRoot" 0 0))
        (Utilities|Array|Add (Variables|Default|GetHandlerList) _returnvalue_5)
        (Transformation|AttachActorToActor _returnvalue_5 self "None" "KeepWorld" "KeepWorld" "KeepWorld" false)
        (Variables|/Game/MIRIEL/Proto_M02/Unit/Squad/SquadSingleUnitHandler.SquadSingleUnitHandler_C|SetUnitToHandle _returnvalue_5 _returnvalue_4)
        (Variables|/Game/MIRIEL/Proto_M02/Unit/Squad/SquadSingleUnitHandler.SquadSingleUnitHandler_C|SetUnitType _returnvalue_5 (.Value (Utilities|Map|Find (Variables|Default|GetSquadFormation) (Math|Vector2D|MakeVector2D (Math|Conversions|ToFloat(Integer) _index_2) (Math|Conversions|ToFloat(Integer) _index)))))))))

(fn ConstructionScript
  (|CallParentFunction)
  (Variables|Default|SetSquadFormation (Variables|/Game/MIRIEL/Proto_M02/Unit/Formation/BPDA_Formation.BPDA_Formation_C|GetFormation%20Layout (Variables|Default|GetFormationDA)))
  (Transformation|SetRelativeLocation (Variables|Default|Getdebug%20indicator) (Math|Vector|MakeVector 0.0 0.0 (Variables|Default|GetSquad%20Height)) false true))

(fn Reassign
  (bind _output_get (LocalVariables|SetUnitToProcess (Variables|Default|GetUnitList)))
  (LocalVariables|SetHandlerToProcess (Variables|Default|GetHandlerList))
  (for _array_element _output_get
    (Variables|/Game/MIRIEL/Proto_M02/Unit/Squad/BPC_SelectableUnitSquadInfo.BPC_SelectableUnitSquadInfo_C|SetDistanceToSquadCenter (Variables|/Game/MIRIEL/Proto_M02/Unit/Old/BP_M02_SelectableUnit_deprecated.BP_M02_SelectableUnit_deprecated_C|GetBPC_SelectableUnitSquadInfo _array_element) (Math|Vector|Distance(Vector) (Transformation|GetActorLocation _array_element) (Variables|Default|GetCurrentProjectedLocation))))
  (while (Utilities|Array|IsNotEmpty (LocalVariables|GetUnitToProcess))
    ;[1 1 1] Setting the first unit as default value
    (LocalVariables|SetmaxDistance (Variables|/Game/MIRIEL/Proto_M02/Unit/Squad/BPC_SelectableUnitSquadInfo.BPC_SelectableUnitSquadInfo_C|GetDistanceToSquadCenter (Variables|/Game/MIRIEL/Proto_M02/Unit/Old/BP_M02_SelectableUnit_deprecated.BP_M02_SelectableUnit_deprecated_C|GetBPC_SelectableUnitSquadInfo (Utilities|Array|Get(acopy) (LocalVariables|GetUnitToProcess)))))
    (LocalVariables|SetfarthestUnit (Utilities|Array|Get(acopy) (LocalVariables|GetUnitToProcess)))
    (LocalVariables|SetUnitIndex 0)
    ;[1 1 1] Search for farthestUnit
    (for (_array_element_2 _array_index) (LocalVariables|GetUnitToProcess)
      (if (> (Variables|/Game/MIRIEL/Proto_M02/Unit/Squad/BPC_SelectableUnitSquadInfo.BPC_SelectableUnitSquadInfo_C|GetDistanceToSquadCenter (Variables|/Game/MIRIEL/Proto_M02/Unit/Old/BP_M02_SelectableUnit_deprecated.BP_M02_SelectableUnit_deprecated_C|GetBPC_SelectableUnitSquadInfo _array_element_2)) (LocalVariables|GetmaxDistance))
        (LocalVariables|SetmaxDistance (Variables|/Game/MIRIEL/Proto_M02/Unit/Squad/BPC_SelectableUnitSquadInfo.BPC_SelectableUnitSquadInfo_C|GetDistanceToSquadCenter (Variables|/Game/MIRIEL/Proto_M02/Unit/Old/BP_M02_SelectableUnit_deprecated.BP_M02_SelectableUnit_deprecated_C|GetBPC_SelectableUnitSquadInfo _array_element_2)))
        (LocalVariables|SetfarthestUnit _array_element_2)
        (LocalVariables|SetUnitIndex _array_index)))
    (LocalVariables|SetfarthestUnitLocation (Transformation|GetActorLocation (LocalVariables|GetfarthestUnit)))
    (LocalVariables|SetNearestHandler 0)
    (for (_array_element_3 _array_index_2) (LocalVariables|GetHandlerToProcess)
      (if (Utilities|ClassIsChildOf (Utilities|GetClass (LocalVariables|GetfarthestUnit)) (Variables|/Game/MIRIEL/Proto_M02/Unit/Squad/SquadSingleUnitHandler.SquadSingleUnitHandler_C|GetUnitType _array_element_3))
        (if (Utilities|IsValid (LocalVariables|GetNearestHandler))
          (if (< (Math|Vector|Distance(Vector) (LocalVariables|GetfarthestUnitLocation) (Variables|/Game/MIRIEL/Proto_M02/Unit/Squad/SquadSingleUnitHandler.SquadSingleUnitHandler_C|GetCurrentLocationToGoTo _array_element_3)) (LocalVariables|GetminDistance))
            (LocalVariables|SetNearestHandler _array_element_3)
            (LocalVariables|SetminDistance (Math|Vector|Distance(Vector) (LocalVariables|GetfarthestUnitLocation) (Variables|/Game/MIRIEL/Proto_M02/Unit/Squad/SquadSingleUnitHandler.SquadSingleUnitHandler_C|GetCurrentLocationToGoTo _array_element_3)))
            (LocalVariables|SetHandlerIndex _array_index_2))
          (else
            ;[1 1 1] Assign First Value to compare for nearest Handler (maybe better putting it before
            (bind _output_get_2 (LocalVariables|SetNearestHandler _array_element_3))
            (LocalVariables|SetminDistance (Math|Vector|Distance(Vector) (Variables|/Game/MIRIEL/Proto_M02/Unit/Squad/SquadSingleUnitHandler.SquadSingleUnitHandler_C|GetCurrentLocationToGoTo _output_get_2) (LocalVariables|GetfarthestUnitLocation)))
            (LocalVariables|SetHandlerIndex _array_index_2)))))
    (Variables|/Game/MIRIEL/Proto_M02/Unit/Squad/SquadSingleUnitHandler.SquadSingleUnitHandler_C|SetUnitToHandle (LocalVariables|GetNearestHandler) (LocalVariables|GetfarthestUnit))
    (LocalVariables|SetfarthestUnit 0)
    (Utilities|Array|RemoveIndex (LocalVariables|GetUnitToProcess) (LocalVariables|GetUnitIndex))
    (LocalVariables|SetNearestHandler 0)
    (Utilities|Array|RemoveIndex (LocalVariables|GetHandlerToProcess) (LocalVariables|GetHandlerIndex))))

(fn SortMap)

(fn OnSelect
  (for _array_element (Variables|Default|GetUnitList)
    (Rendering|SetVisibility (Variables|/Game/MIRIEL/Proto_M02/Unit/Old/BP_M02_SelectableUnit_deprecated.BP_M02_SelectableUnit_deprecated_C|GetSelection%20Marker _array_element) true false)))

(fn OnUnselect
  (for _array_element (Variables|Default|GetUnitList)
    (Rendering|SetVisibility (Variables|/Game/MIRIEL/Proto_M02/Unit/Old/BP_M02_SelectableUnit_deprecated.BP_M02_SelectableUnit_deprecated_C|GetSelection%20Marker _array_element) false false)))