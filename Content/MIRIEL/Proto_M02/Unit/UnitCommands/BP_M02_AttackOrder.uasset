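; Unit command that sends a unit to attack an enemy squad by moving it toward a target unit's location.
; RefreshTarget picks the closest valid unit in the target squad and re-executes, or finishes if the squad is invalid or empty.
; Interrupt stops movement, and Resume moves again or retargets if the target is gone.
; Finish teleports the parent squad to the unit, calls its MoveAllUnitV2 and pops the command from the stack.
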(fn `Execute`
  (bind _correspondingunit (`self.CorrespondingUnit`))
  (`parent.Execute`)
  (`/Game/MIRIEL/Proto_M02/Unit/Old/BP_M02_SelectableUnit_deprecated.Move To` _correspondingunit (`Actor.K2_GetActorLocation` (`self.TargetUnit`)) self (`/Game/MIRIEL/Proto_M02/Unit/Old/BP_M02_SelectableUnit_deprecated.CurrentHandler` _correspondingunit)))

(fn `Finish`
  (bind _correspondingunit (`self.CorrespondingUnit`))
  (bind _returnvalue (`Actor.GetTransform` _correspondingunit))
  (bind _parentsquad (`/Game/MIRIEL/Proto_M02/Unit/Old/BP_M02_SelectableUnit_deprecated.ParentSquad` _correspondingunit))
  (bind (_returnvalue_x _returnvalue_y _returnvalue_z) (`KismetMathLibrary.BreakVector` (`Actor.K2_GetActorLocation` _parentsquad)))
  (`parent.Finish`)
  (`Actor.K2_SetActorLocationAndRotation` _parentsquad (`KismetMathLibrary.MakeVector` (.x (.location _returnvalue)) (.y (.location _returnvalue)) _returnvalue_z) (.rotation _returnvalue) false true)
  (`/Game/MIRIEL/Proto_M02/Unit/Squad/BP_M02_Squad_Default.Move All Unit V2` _parentsquad)
  (`/Game/MIRIEL/Proto_M02/Unit/UnitCommands/BPC_UnitCommandStack.Pop Command by Object` (`self.CurrentStack`) self))

(fn `Interrupt`
  (if (not (`self.isInterrupted`))
    (set `self.isInterrupted` true)
    (`MovementComponent.StopMovementImmediately` (`Character.CharacterMovement` (`self.CorrespondingUnit`)))))

(fn `Pause`
  (`parent.Pause`))

(fn `RefreshTarget`
  (locals (MinDistance :type "Float (double-precision)" :default 0.0))
  (bind _unitlist (`/Game/MIRIEL/Proto_M02/Unit/Squad/BP_M02_Squad_Default.UnitList` (`self.TargetSquad`)))
  (if (`KismetSystemLibrary.IsValid` (`self.TargetSquad`))
    (if (`KismetArrayLibrary.Array_IsNotEmpty` _unitlist)
      (bind _output_get (set `self.TargetUnit` (`|GetArrayItem` _unitlist)))
      (set `local.MinDistance` (`KismetMathLibrary.Vector_Distance` (`Actor.K2_GetActorLocation` _output_get) (`Actor.K2_GetActorLocation` (`self.CorrespondingUnit`))))
      (for _array_element _unitlist
        (if (`KismetSystemLibrary.IsValid` _array_element)
          (bind _returnvalue (`KismetMathLibrary.Vector_Distance` (`Actor.K2_GetActorLocation` _array_element) (`Actor.K2_GetActorLocation` (`self.CorrespondingUnit`))))
          (if (< _returnvalue (`local.MinDistance`))
            (set `self.TargetUnit` _array_element)
            (set `local.MinDistance` _returnvalue))))
      (`self.Execute`)
      (else
        (`self.Finish` :!label _label)))
    (else
      (goto _label))))

(fn `Resume`
  (bind _targetunit (`self.TargetUnit`))
  (bind _correspondingunit (`self.CorrespondingUnit`))
  (`parent.Resume`)
  (if (`KismetSystemLibrary.IsValid` _targetunit)
    (`/Game/MIRIEL/Proto_M02/Unit/Old/BP_M02_SelectableUnit_deprecated.Move To` _correspondingunit (`Actor.K2_GetActorLocation` _targetunit) self (`/Game/MIRIEL/Proto_M02/Unit/Old/BP_M02_SelectableUnit_deprecated.CurrentHandler` _correspondingunit))
    (else
      (`self.RefreshTarget`))))

(fn `Unpause`
  (`parent.Unpause`))

(fn `UpdateOnTenth`
  (`parent.UpdateOnTenth`))