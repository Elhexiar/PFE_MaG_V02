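; Blueprint component that holds a list of unit command objects as a stack, with index 0 as the top.
; Adding a command executes it first, then inserts it at a given index and stores that index and a stack back-reference on it.
; Commands are removed from the top, by object, by index or all at once, with no other calls on them.
; A separate function renumbers stored indices, but the add and remove functions do not call it.
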(fn `Add New Command`
  (params (`New Command` :type "/Game/MIRIEL/Proto_M02/Unit/UnitCommands/BP_M02_UnitCommand Object Reference") (NewParam :type Integer))
  (`/Game/MIRIEL/Proto_M02/Unit/UnitCommands/BP_M02_UnitCommand.Execute` `New Command`)
  (`KismetArrayLibrary.Array_Insert` (`self.CommandList`) `New Command` NewParam)
  (set `/Game/MIRIEL/Proto_M02/Unit/UnitCommands/BP_M02_UnitCommand.StackIndex` NewParam `New Command`)
  (set `/Game/MIRIEL/Proto_M02/Unit/UnitCommands/BP_M02_UnitCommand.CurrentStack` self `New Command`))

(fn `ClearCommandList`
  (`KismetArrayLibrary.Array_Clear` (`self.CommandList`)))

(fn `Pop Command by Index`
  (params (`Command index` :type Integer))
  (`KismetArrayLibrary.Array_Remove` (`self.CommandList`) `Command index`))

(fn `Pop Command by Object`
  (params (`Command index` :type "/Game/MIRIEL/Proto_M02/Unit/UnitCommands/BP_M02_UnitCommand Object Reference"))
  (`KismetArrayLibrary.Array_RemoveItem` (`self.CommandList`) `Command index`))

(fn `Pop Top Command`
  (`self.Pop Command by Index` 0))

(fn `UpdateCommandIndex`
  (for (_array_element _array_index) (`self.CommandList`)
    (set `/Game/MIRIEL/Proto_M02/Unit/UnitCommands/BP_M02_UnitCommand.StackIndex` _array_index _array_element)))