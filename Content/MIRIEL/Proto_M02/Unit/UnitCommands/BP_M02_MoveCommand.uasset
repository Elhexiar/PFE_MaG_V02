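; Unit command for the M02 prototype that sends its unit to a destination location as part of a command stack.
; Execute, Resume and Unpause (unless interrupted) call the unit's MoveTo, passing the command and its handler.
; Pause and Interrupt set their flags and halt character movement immediately, while Finish pops the command off the current stack.
; UpdateOnTenth prints the handler's unit name after a validity check.
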(fn `Execute`
  (`parent.Execute`)
  (`/Game/MIRIEL/Proto_M02/Unit/Old/BP_M02_SelectableUnit_deprecated.Move To` (`self.CorrespondingUnit`) (`self.DestinationLocation`) self (`self.Handler`)))

(fn `Finish`
  (`parent.Finish`)
  (`/Game/MIRIEL/Proto_M02/Unit/UnitCommands/BPC_UnitCommandStack.Pop Command by Object` (`self.CurrentStack`) self))

(fn `Interrupt`
  (if (not (`self.isInterrupted`))
    (set `self.isInterrupted` true)
    (`MovementComponent.StopMovementImmediately` (`Character.CharacterMovement` (`self.CorrespondingUnit`)))))

(fn `Pause`
  (if (not (`self.isPaused`))
    (set `self.isPaused` true)
    (`MovementComponent.StopMovementImmediately` (`Character.CharacterMovement` (`self.CorrespondingUnit`)))))

(fn `Resume`
  (`parent.Resume`)
  (`/Game/MIRIEL/Proto_M02/Unit/Old/BP_M02_SelectableUnit_deprecated.Move To` (`self.CorrespondingUnit`) (`self.DestinationLocation`) self (`self.Handler`)))

(fn `Unpause`
  (`parent.Unpause`)
  (if (not (`self.isInterrupted`))
    (`/Game/MIRIEL/Proto_M02/Unit/Old/BP_M02_SelectableUnit_deprecated.Move To` (`self.CorrespondingUnit`) (`self.DestinationLocation`) self (`self.Handler`))))

(fn `UpdateOnTenth`
  (`parent.UpdateOnTenth`)
  (if (`self.isValid`)
    (`KismetSystemLibrary.PrintString` null (`KismetSystemLibrary.GetDisplayName` (`/Game/MIRIEL/Proto_M02/Unit/Squad/BP_M02_Handler.UnitToHandle` (`self.Handler`))))))