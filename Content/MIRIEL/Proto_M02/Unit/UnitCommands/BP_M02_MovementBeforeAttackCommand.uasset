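; BP_M02_MovementBeforeAttackCommand is a unit command in the M02 prototype, named for the movement step that precedes an attack.
; It overrides the command lifecycle (Execute, Finish, Interrupt, Pause, Resume, Unpause) and UpdateOnTenth.
; Each override only calls its parent, so the graphs add no logic and all behavior comes from the parent class.
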(fn `Execute`
  (`parent.Execute`))

(fn `Finish`
  (`parent.Finish`))

(fn `Interrupt`
  (`parent.Interrupt`))

(fn `Pause`
  (`parent.Pause`))

(fn `Resume`
  (`parent.Resume`))

(fn `Unpause`
  (`parent.Unpause`))

(fn `UpdateOnTenth`
  (`parent.UpdateOnTenth`))