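; BP_M02_SpeedBuff is a timed-effect style Hedif buff that changes the afflicted unit's speed while active.
; OnStart calls the parent, then adds SpeedAmount through the unit's UnitStatComponent.
; OnFinish calls the parent, adds the negated amount to undo the change, and sets IsFinished.
; Both events print a debug string.
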(fn `OnFinish`
  (`parent.OnFinish`)
  (`/Game/MIRIEL/Proto_M02/Unit/Old/M02_BPC_UnitStatComponent.AddSpeed` (`/Game/MIRIEL/Proto_M02/Unit/Old/BP_M02_SelectableUnit_deprecated.UnitStatComponent` (`self.AfflictedUnit`)) (* (`self.SpeedAmount`) -1.0))
  (`KismetSystemLibrary.PrintString` null "finish speed buff")
  (set `self.isFinished` true))

(fn `OnStart`
  (`parent.OnStart`)
  (`/Game/MIRIEL/Proto_M02/Unit/Old/M02_BPC_UnitStatComponent.AddSpeed` (`/Game/MIRIEL/Proto_M02/Unit/Old/BP_M02_SelectableUnit_deprecated.UnitStatComponent` (`self.AfflictedUnit`)) (`self.SpeedAmount`))
  (`KismetSystemLibrary.PrintString` null "start speed buff"))