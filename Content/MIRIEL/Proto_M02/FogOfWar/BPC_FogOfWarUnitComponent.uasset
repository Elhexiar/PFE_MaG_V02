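; Unit component that paints its owner's position into a fog of war render target.
; BeginPlay creates a dynamic instance of the fog render material and caches the M02 RTS player controller.
; Each Tick it line traces down from the owner, reads the hit UV as the material's Location, and draws the material to the render target.
; Mapping relies on collision UVs rather than world coordinates.
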(event `self.ReceiveBeginPlay`
  (bind _asbp_m02_rtscontroler (`/Game/MIRIEL/Proto_M02/Utils/BPFL_M02_Utils.Get_M02_PlayerController`))
  (set `self.BP M02 RTSControler` _asbp_m02_rtscontroler)
  (bind _returnvalue (`KismetMaterialLibrary.CreateDynamicMaterialInstance` "/Game/MIRIEL/Proto_M02/FogOfWar/M_FogRenderMaterial.M_FogRenderMaterial"))
  (set `self.FogOfWarMaterialDynInstance` _returnvalue))

(event `self.ReceiveTick`
  (params (DeltaSeconds :type "Float (single-precision)"))
  (bind _returnvalue (`Actor.K2_GetActorLocation` (`self.GetOwner`)))
  (bind _outhit (`KismetSystemLibrary.LineTraceSingle` _returnvalue (- _returnvalue (0.0 0.0 1000.0)) "TraceTypeQuery6" true))
  (bind _uv (`GameplayStatics.FindCollisionUV` _outhit))
  (`MaterialInstanceDynamic.SetVectorParameterValue` (`self.FogOfWarMaterialDynInstance`) "Location" (make `LinearColor` (`KismetMathLibrary.BreakVector2D` _uv) (`.Y` (`KismetMathLibrary.BreakVector2D` _uv)) 0.0 1.0))
  (`KismetRenderingLibrary.DrawMaterialToRenderTarget` "/Game/MIRIEL/Proto_M02/FogOfWar/FogOfWarRender.FogOfWarRender" (`self.FogOfWarMaterialDynInstance`)))