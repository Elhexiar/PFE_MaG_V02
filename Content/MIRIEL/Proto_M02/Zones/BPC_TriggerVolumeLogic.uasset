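; Capture-zone component for a BP_CustomTriggerVolume that tracks overlapping squads and generates resources for team 0.
; Overlap events update unit and squad lists, recording only the first unit of each new squad.
; UpdateSquadList derives contested, captured or empty state, taking TeamID from a lone squad.
; Tick advances a delivery timer whenever TeamID is 0, calling the player resource manager every tick past the threshold, as only contested or empty updates reset it.
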(event `self.ReceiveBeginPlay`
  (bind _asbp_m02_rtscontroler (`/Game/MIRIEL/Proto_M02/Utils/BPFL_M02_Utils.Get_M02_PlayerController`))
  (set `self.BP M02 RTSControler` _asbp_m02_rtscontroler)
  (bind _asbp_custom_trigger_volume (cast `/Game/MIRIEL/Proto_M02/Zones/BP_CustomTriggerVolume` (`self.GetOwner`)))
  (bind _output_get (set `self.Custom Trigger Volume` _asbp_custom_trigger_volume))
  (add `Actor.OnActorBeginOverlap` _output_get (delegate `OnActorBeginOverlap_Event`))
  (add `Actor.OnActorEndOverlap` _output_get (delegate `OnActorEndOverlap_Event`)))

(event `OnActorEndOverlap_Event`
  (params (OverlappedActor :type "Actor Object Reference") (OtherActor :type "Actor Object Reference"))
  (bind _asbp_m02_selectable_unit_deprecated (cast `/Game/MIRIEL/Proto_M02/Unit/Old/BP_M02_SelectableUnit_deprecated` OtherActor))
  (`KismetArrayLibrary.Array_RemoveItem` (`self.UnitList`) _asbp_m02_selectable_unit_deprecated)
  (`self.UpdateSquadList`))

(event `OnActorBeginOverlap_Event`
  (params (OverlappedActor :type "Actor Object Reference") (OtherActor :type "Actor Object Reference"))
  (bind _squadlist (`self.SquadList`))
  (bind _asbp_m02_selectable_unit_deprecated (cast `/Game/MIRIEL/Proto_M02/Unit/Old/BP_M02_SelectableUnit_deprecated` OtherActor))
  (bind _parentsquad (`/Game/MIRIEL/Proto_M02/Unit/Old/BP_M02_SelectableUnit_deprecated.ParentSquad` _asbp_m02_selectable_unit_deprecated))
  (if (not (`KismetArrayLibrary.Array_Contains` _squadlist _parentsquad))
    (`KismetArrayLibrary.Array_AddUnique` _squadlist _parentsquad)
    (`KismetArrayLibrary.Array_Add` (`self.UnitList`) _asbp_m02_selectable_unit_deprecated)
    (`self.UpdateSquadList`)))

(event `self.ReceiveTick`
  (params (DeltaSeconds :type "Float (single-precision)"))
  (if (== (`self.TeamID`) 0)
    (bind _output_get (set `self.CurrentDeliveryTime` (+ DeltaSeconds (`self.CurrentDeliveryTime`))))
    (if (>= _output_get (`self.MaxDeliveryTime`))
      (`self.TriggerRessourceGeneration`))))

(event `TriggerRessourceGeneration`
  (`/Game/MIRIEL/Proto_M02/Player/BPC_PlayerRessourceManager.AddRessource` (`/Game/MIRIEL/Proto_M02/Player/BP_M02_RTSControler.BPC_PlayerRessourceManager` (`self.BP M02 RTSControler`)) 0))

(fn `UpdateSquadList`
  (locals (SquadIsPresent :type Boolean))
  (for _array_element (`self.SquadList`)
    (set `local.SquadIsPresent` false)
    (for _array_element_2 (`self.UnitList`)
      (if (== (`/Game/MIRIEL/Proto_M02/Unit/Old/BP_M02_SelectableUnit_deprecated.ParentSquad` _array_element_2) _array_element)
        (set `local.SquadIsPresent` true)
        (break)))
    (if (not (`local.SquadIsPresent`))
      (`KismetArrayLibrary.Array_RemoveItem` (`self.SquadList`) _array_element)))
  (if (> (`KismetArrayLibrary.Array_Length` (`self.SquadList`)) 1)
    ;[1 1 1] Enum + Struct ?
    (set `self.Contested` true)
    (set `self.Captured` false)
    (set `self.Empty` false)
    (set `self.CurrentDeliveryTime` 0.0)
    (elif (== (`KismetArrayLibrary.Array_Length` (`self.SquadList`)) 1)
      (set `self.Contested` false)
      (set `self.Captured` true)
      (set `self.Empty` false)
      (set `self.TeamID` (`/Game/MIRIEL/Proto_M02/Unit/Squad/BP_M02_Squad_Default.TeamNumber` (`|GetArrayItem` (`self.SquadList`))))
      (elif (< (`KismetArrayLibrary.Array_Length` (`self.SquadList`)) 1)
        (set `self.Contested` false)
        (set `self.Captured` false)
        (set `self.Empty` true)
        (set `self.CurrentDeliveryTime` 0.0)))))