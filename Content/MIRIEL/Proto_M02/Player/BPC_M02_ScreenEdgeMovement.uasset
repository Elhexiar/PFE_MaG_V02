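; Player component for the M02 prototype that adds screen-edge scrolling to move the camera with the mouse.
; Each tick it compares the cursor position to border zones sized as fractions of the viewport and sums a direction vector, allowing diagonals at corners.
; It injects that vector into the Enhanced Input camera move action every frame, zero included, rather than moving the camera directly.
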(event `self.ReceiveBeginPlay`
  (set `self.PlayerControler` (`GameplayStatics.GetPlayerController` 0)))

(event `self.ReceiveTick`
  (params (DeltaSeconds :type "Float (single-precision)"))
  (bind _returnvalue_x (`KismetMathLibrary.BreakVector2D` (`WidgetLayoutLibrary.GetViewportSize`)))
  (bind _returnvalue_x_2 (`KismetMathLibrary.BreakVector2D` (`WidgetLayoutLibrary.GetViewportSize`)))
  (bind (_returnvalue_x_3 _returnvalue_y) (`KismetMathLibrary.BreakVector2D` (`WidgetLayoutLibrary.GetViewportSize`)))
  (bind (_returnvalue_x_4 _returnvalue_y_2) (`KismetMathLibrary.BreakVector2D` (`WidgetLayoutLibrary.GetViewportSize`)))
  (bind _output_get (set `self.Camera Border Movement Vector` (0.0 0.0 0.0)))
  (if (<= (`.LocationY` (`PlayerController.GetMousePosition` (`self.PlayerControler`))) (* _returnvalue_y (`self.VerticalBorderDeadZone`)))
    (bind _output_get_2 (set `self.Camera Border Movement Vector` (+ _output_get (0.0 1.0 0.0)))))
  (if (>= (`.LocationY` (`PlayerController.GetMousePosition` (`self.PlayerControler`))) (- _returnvalue_y_2 (* _returnvalue_y_2 (`self.VerticalBorderDeadZone`))))
    (bind _output_get_3 (set `self.Camera Border Movement Vector` (+ _output_get_2 (0.0 -1.0 0.0)))))
  (if (<= (`PlayerController.GetMousePosition` (`self.PlayerControler`)) (* _returnvalue_x_2 (`self.HorizontalBorderDeadZone`)))
    (bind _output_get_4 (set `self.Camera Border Movement Vector` (+ _output_get_3 (-1.0 0.0 0.0)))))
  (if (>= (`PlayerController.GetMousePosition` (`self.PlayerControler`)) (- _returnvalue_x (* _returnvalue_x (`self.HorizontalBorderDeadZone`))))
    (bind _output_get_5 (set `self.Camera Border Movement Vector` (+ _output_get_4 (1.0 0.0 0.0)))))
  (`EnhancedInputSubsystemInterface.InjectInputVectorForAction` :`self` (pcsubsystem `EnhancedInputLocalPlayerSubsystem` (`self.PlayerControler`)) :`Action` "/Game/MIRIEL/Proto_M02/Input/IA_M02_CameraMove.IA_M02_CameraMove" :`Value` _output_get_5))