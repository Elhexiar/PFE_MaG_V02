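; BPC_PlayerRessourceManager is a player component that tracks a current resource amount against a maximum.
; AddRessource adds an amount, clamps the total to the maximum and prints the current and max values as debug text.
; RemoveRessource is an empty stub, and the BeginPlay and Tick events do nothing.
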(fn `AddRessource`
  (params (RessourceAmount :type Integer))
  (bind _returnvalue (+ RessourceAmount (`self.CurrentRessources`)))
  (if (> _returnvalue (`self.MaxRessources`))
    (set `self.CurrentRessources` (`self.MaxRessources`))
    (else
      (bind _output_get (set `self.CurrentRessources` _returnvalue))))
  (`KismetSystemLibrary.PrintString` (`KismetStringLibrary.Concat_StrStr` "PlayerRessource = " (`KismetStringLibrary.Conv_IntToString` _output_get) "/" (`KismetStringLibrary.Conv_IntToString` (`self.MaxRessources`)))))

(fn `RemoveRessource`)