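; Card manager component for the M02 prototype that creates the card pool and the player's deck at BeginPlay.
; It converts a list of data assets into summon or active card objects, casting active ones to damage zone, speed buff or draw card types.
; The player deck holds 30 random picks from that overall deck, with repeats possible and sharing the same card objects.
; Building a deck from a card list is only a stub.
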(event `self.ReceiveBeginPlay`
  (bind _asbp_m02_rtscontroler (`/Game/MIRIEL/Proto_M02/Utils/BPFL_M02_Utils.Get_M02_PlayerController`))
  (set `self.As BP M02 RTSControler` _asbp_m02_rtscontroler)
  (`|ExecutionSequence`
    (:`then_0`
      (bind _deck (`self.BuildDeckFromDAList` (`self.generalDA_CardList`)))
      (set `self.OverallDeck` _deck))
    (:`then_1`
      (bind _built_deck (`self.BuildDeckWithNRandomCards` 30))
      (set `self.CurrentPlayerDeck` _built_deck))))

(fn `Build Active Card from DA`
  (params (dataAsset :type "/Game/MIRIEL/Proto_M02/Cards/BPDA/BPDA_M02_ActiveCard Object Reference"))
  (returns (activeCard :type "/Game/MIRIEL/Proto_M02/Cards/BP_M02_ActiveCard Object Reference"))
  (locals (DataAssetToBuildFrom :type "/Game/MIRIEL/Proto_M02/Cards/BPDA/BPDA_M02_ActiveCard Object Reference"))
  (bind _output_get (set `local.DataAssetToBuildFrom` dataAsset))
  (bind _asbpda_m02__temp_dammage_zone (cast `/Game/MIRIEL/Proto_M02/Cards/BPDA/BPDA_M02__Temp_DammageZone` _output_get)
    (:`then`
      (bind _returnvalue (`|GenericCreateObject` "/Game/MIRIEL/Proto_M02/Cards/BP_M02_Temp_DamageZoneCard.BP_M02_Temp_DamageZoneCard_C" (`/Game/MIRIEL/Proto_M02/Cards/BPDA/BPDA_M02__Temp_DammageZone.Damage` _asbpda_m02__temp_dammage_zone) (`/Game/MIRIEL/Proto_M02/Cards/BPDA/BPDA_M02__Temp_DammageZone.Radius` _asbpda_m02__temp_dammage_zone) (`/Game/MIRIEL/Proto_M02/Cards/BPDA/BPDA_M02__Temp_DammageZone.VFXClass` _asbpda_m02__temp_dammage_zone) (`self.As BP M02 RTSControler`) (`/Game/MIRIEL/Proto_M02/Cards/BPDA/BPDA_M02_ActiveCard.ColorTest2` _asbpda_m02__temp_dammage_zone) (`/Game/MIRIEL/Proto_M02/Cards/BPDA/BPDA_M02_Card.CentralImage` _asbpda_m02__temp_dammage_zone) (`/Game/MIRIEL/Proto_M02/Cards/BPDA/BPDA_M02_Card.Name` _asbpda_m02__temp_dammage_zone) (`/Game/MIRIEL/Proto_M02/Cards/BPDA/BPDA_M02_Card.Cost` _asbpda_m02__temp_dammage_zone) (`/Game/MIRIEL/Proto_M02/Cards/BPDA/BPDA_M02_Card.Description` _asbpda_m02__temp_dammage_zone) (`/Game/MIRIEL/Proto_M02/Cards/BPDA/BPDA_M02_Card.InHandModel` _asbpda_m02__temp_dammage_zone)))
      (return _returnvalue))
    (:`CastFailed`
      (bind _asbpda_m02__temp_speed_upgrade (cast `/Game/MIRIEL/Proto_M02/Cards/BPDA/BPDA_M02__Temp_SpeedUpgrade` _output_get)
        (:`then`
          (bind _returnvalue_2 (`|GenericCreateObject` "/Game/MIRIEL/Proto_M02/Cards/BP_M02_Temp_SpeedBuffCard.BP_M02_Temp_SpeedBuffCard_C" (`/Game/MIRIEL/Proto_M02/Cards/BPDA/BPDA_M02__Temp_SpeedUpgrade.SpeedAmount` _asbpda_m02__temp_speed_upgrade) (`/Game/MIRIEL/Proto_M02/Cards/BPDA/BPDA_M02__Temp_SpeedUpgrade.BuffDuration` _asbpda_m02__temp_speed_upgrade) (`self.As BP M02 RTSControler`) (`/Game/MIRIEL/Proto_M02/Cards/BPDA/BPDA_M02_ActiveCard.ColorTest2` _asbpda_m02__temp_speed_upgrade) (`/Game/MIRIEL/Proto_M02/Cards/BPDA/BPDA_M02_Card.CentralImage` _asbpda_m02__temp_speed_upgrade) (`/Game/MIRIEL/Proto_M02/Cards/BPDA/BPDA_M02_Card.Name` _asbpda_m02__temp_speed_upgrade) (`/Game/MIRIEL/Proto_M02/Cards/BPDA/BPDA_M02_Card.Cost` _asbpda_m02__temp_speed_upgrade) (`/Game/MIRIEL/Proto_M02/Cards/BPDA/BPDA_M02_Card.Description` _asbpda_m02__temp_speed_upgrade) (`/Game/MIRIEL/Proto_M02/Cards/BPDA/BPDA_M02_Card.InHandModel` _asbpda_m02__temp_speed_upgrade)))
          (return _returnvalue_2))
        (:`CastFailed`
          (bind _asbpda_m02__temp_draw_card (cast `/Game/MIRIEL/Proto_M02/Cards/BPDA/BPDA_M02__Temp_DrawCard` _output_get)
            (:`then`
              (bind _returnvalue_3 (`|GenericCreateObject` "/Game/MIRIEL/Proto_M02/Cards/BP_M02_Temp_DrawCard.BP_M02_Temp_DrawCard_C" (`/Game/MIRIEL/Proto_M02/Cards/BPDA/BPDA_M02__Temp_DrawCard.NumberOfDraw` _asbpda_m02__temp_draw_card) (`self.As BP M02 RTSControler`) (`/Game/MIRIEL/Proto_M02/Cards/BPDA/BPDA_M02_ActiveCard.ColorTest2` _asbpda_m02__temp_draw_card) (`/Game/MIRIEL/Proto_M02/Cards/BPDA/BPDA_M02_Card.CentralImage` _asbpda_m02__temp_draw_card) (`/Game/MIRIEL/Proto_M02/Cards/BPDA/BPDA_M02_Card.Name` _asbpda_m02__temp_draw_card) (`/Game/MIRIEL/Proto_M02/Cards/BPDA/BPDA_M02_Card.Cost` _asbpda_m02__temp_draw_card) (`/Game/MIRIEL/Proto_M02/Cards/BPDA/BPDA_M02_Card.Description` _asbpda_m02__temp_draw_card) (`/Game/MIRIEL/Proto_M02/Cards/BPDA/BPDA_M02_Card.InHandModel` _asbpda_m02__temp_draw_card)))
              (return _returnvalue_3))
            (:`CastFailed`
              (`KismetSystemLibrary.PrintString` "ActiveCard Type not recognised"))))))))

(fn `Build Deck from Card List`
  (`KismetSystemLibrary.PrintString` "Build Deck from Card List not implemented yet"))

(fn `BuildDeckFromDAList`
  (params (dataAssetList :type "Array of /Game/MIRIEL/Proto_M02/Cards/BPDA/BPDA_M02_Card Object Reference"))
  (returns (Deck :type "/Game/MIRIEL/Proto_M02/Cards/BP_M02_Deck Object Reference"))
  (bind _returnvalue (`|GenericCreateObject` "/Game/MIRIEL/Proto_M02/Cards/BP_M02_Deck.BP_M02_Deck_C"))
  (for _array_element dataAssetList
    (bind _asbpda_m02_summon_card (cast `/Game/MIRIEL/Proto_M02/Cards/BPDA/BPDA_M02_SummonCard` _array_element)
      (:`then`
        (bind _summoncard (`self.BuildSummonCardFromDA` _asbpda_m02_summon_card))
        (`/Game/MIRIEL/Proto_M02/Cards/BP_M02_Deck.AddTopCard` _returnvalue _summoncard))
      (:`CastFailed`
        (bind _asbpda_m02_active_card (cast `/Game/MIRIEL/Proto_M02/Cards/BPDA/BPDA_M02_ActiveCard` _array_element))
        (bind _activecard (`self.Build Active Card from DA` _asbpda_m02_active_card))
        (`/Game/MIRIEL/Proto_M02/Cards/BP_M02_Deck.AddTopCard` _returnvalue _activecard))))
  (return _returnvalue))

(fn `BuildDeckWithNRandomCards`
  (params (`n size` :type Integer))
  (returns (`Built Deck` :type "/Game/MIRIEL/Proto_M02/Cards/BP_M02_Deck Object Reference"))
  (bind _cardlist (`/Game/MIRIEL/Proto_M02/Cards/BP_M02_Deck.cardList` (`self.OverallDeck`)))
  (bind _returnvalue (`|GenericCreateObject` "/Game/MIRIEL/Proto_M02/Cards/BP_M02_Deck.BP_M02_Deck_C"))
  (for _ (range 1 (+ `n size` 1))
    (`/Game/MIRIEL/Proto_M02/Cards/BP_M02_Deck.AddCardAtRandomIndex` _returnvalue (`|GetArrayItem` _cardlist (`.OutIndex` (`KismetArrayLibrary.Array_Random` _cardlist)))))
  (return _returnvalue))

(fn `BuildSummonCardFromDA`
  (params (dataAsset :type "/Game/MIRIEL/Proto_M02/Cards/BPDA/BPDA_M02_SummonCard Object Reference"))
  (returns (summonCard :type "/Game/MIRIEL/Proto_M02/Cards/BP_M02_SummonCard Object Reference"))
  (locals (DataAssetToBuildFrom :type "/Game/MIRIEL/Proto_M02/Cards/BPDA/BPDA_M02_SummonCard Object Reference"))
  (bind _output_get (set `local.DataAssetToBuildFrom` dataAsset))
  (bind _returnvalue (`|GenericCreateObject` "/Game/MIRIEL/Proto_M02/Cards/BP_M02_SummonCard.BP_M02_SummonCard_C" (`/Game/MIRIEL/Proto_M02/Cards/BPDA/BPDA_M02_SummonCard.TestColor` _output_get) (`/Game/MIRIEL/Proto_M02/Cards/BPDA/BPDA_M02_SummonCard.FormationToSpawn` _output_get) (`/Game/MIRIEL/Proto_M02/Cards/BPDA/BPDA_M02_Card.CentralImage` _output_get) (`/Game/MIRIEL/Proto_M02/Cards/BPDA/BPDA_M02_Card.Name` _output_get) (`/Game/MIRIEL/Proto_M02/Cards/BPDA/BPDA_M02_Card.Cost` _output_get) (`/Game/MIRIEL/Proto_M02/Cards/BPDA/BPDA_M02_Card.Description` _output_get) (`/Game/MIRIEL/Proto_M02/Cards/BPDA/BPDA_M02_Card.InHandModel` _output_get)))
  (return _returnvalue))