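; BP_Charriot is a cart actor that travels along a spline from start to end once play begins.
; On BeginPlay it finds a BP_splineTest actor in the level, stores it and starts the move event.
; The MoveCharriot timeline, with play rate scaled by 1/TimeToComplete, lerps distance over the spline's length.
; Each update sets the actor's location and rotation from the spline in world space.
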(event `self.ReceiveBeginPlay`
  (bind _returnvalue (`GameplayStatics.GetActorOfClass` "/Game/BODERE/BP_splineTest.BP_splineTest_C"))
  (set `self.splineREF` _returnvalue)
  (`self.moveEvent`))

(event `moveEvent`
  (bind _spline (`/Game/BODERE/BP_splineTest.Spline` (`self.splineREF`)))
  (`TimelineComponent.SetPlayRate` (`self.MoveCharriot`) (/ 1.0 (`self.timeToComplete`)))
  (bind (_direction _movet) (`Timeline|MoveCharriot`)
    (:`Update`
      (bind _returnvalue (`KismetMathLibrary.Lerp` 0.0 (`SplineComponent.GetSplineLength` (`/Game/BODERE/BP_splineTest.Spline` (`self.splineREF`))) _movet))
      (`self.K2_SetActorTransform` (`KismetMathLibrary.MakeTransform` (`SplineComponent.GetLocationAtDistanceAlongSpline` _spline _returnvalue "World") (`SplineComponent.GetRotationAtDistanceAlongSpline` _spline _returnvalue "World"))))))

(fn `UserConstructionScript`)